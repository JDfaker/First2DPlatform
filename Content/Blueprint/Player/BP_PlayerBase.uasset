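; BP_PlayerBase is a player Character Blueprint that handles basic movement and jump input.
; The MoveRight axis adds movement input along the control rotation's forward vector, not its right vector.
; Pressing Jump calls the character jump only when a helper function confirms the movement component is not falling.
; BeginPlay is empty and the construction script only calls its parent.
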(event EventBeginPlay)

(event Input|ActionEvents|InputActionJump
  (params (Key :type Key%20Structure :default "None"))
  (:Pressed
    (bind _returnvalue (CallFunction|FIsNotFalling))
    (if _returnvalue
      (Character|Jump))))

(event Input|AxisEvents|InputAxisMoveRight
  (params (AxisValue :type Float%20%28single-precision%29))
  (Pawn|Input|AddMovementInput (Math|Vector|GetForwardVector (Pawn|GetControlRotation :!class /Script/Engine.Pawn)) AxisValue false))

(fn ConstructionScript
  (|CallParentFunction))

(fn FIsNotFalling
  (return (not (AI|Components|NavMovement|IsFalling (Variables|Character|GetCharacterMovement)))))